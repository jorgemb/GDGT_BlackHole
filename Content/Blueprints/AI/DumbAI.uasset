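; DumbAI is a simple AI opponent that sends units between planets at random.
; Tick calls the parent, accumulates time and acts whenever the elapsed time reaches WaitTime.
; Each action picks a random planet from OwnedPlanets and, if it is valid, sends its units to a random one from NotOwnedPlanets.
; This file does not fill either planet list, and only the source planet is validity-checked.
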(event `self.ReceiveTick`
  (params (DeltaSeconds :type "Float (single-precision)"))
  (`parent.ReceiveTick` DeltaSeconds)
  (set `self.CurrentWaitTime` (+ (`self.CurrentWaitTime`) DeltaSeconds))
  (if (>= (`self.CurrentWaitTime`) (`self.WaitTime`))
    (set `self.CurrentWaitTime` 0.0)
    (bind _planet (`self.GetRandomPlanet` (`self.OwnedPlanets`)))
    (`/Engine/EditorBlueprintResources/StandardMacros.IsValid` _planet
      (:`Is Valid`
        (bind _planet_2 (`self.GetRandomPlanet` (`self.NotOwnedPlanets`)))
        (`Planet.SendUnitsToTarget` _planet _planet_2)))))

(fn `GetRandomPlanet`
  (params (PlanetArray :type "Array of Planet Object Reference"))
  (returns (Planet :type "Planet Object Reference"))
  (return (`|GetArrayItem` PlanetArray (`KismetMathLibrary.RandomInteger` (`KismetArrayLibrary.Array_Length` PlanetArray)))))

(fn `UserConstructionScript`)