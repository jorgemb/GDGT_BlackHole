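; AI Blueprint for a planet-conquest game that attacks the closest planet it does not own.
; Each tick, after the parent's tick, the first owned planet at or above the minimum occupancy ratio sends units to the target from GetClosestNotOwnedPlanet.
; That search compares distances over NotOwnedPlanets but starts its closest distance at zero, so as written it never selects a planet.
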(event `self.ReceiveTick`
  (params (DeltaSeconds :type "Float (single-precision)"))
  (`parent.ReceiveTick` DeltaSeconds)
  (for _array_element (`self.OwnedPlanets`)
    (if (>= (`self.GetPlanetOccupancyRatio` _array_element) (`self.MinOccupancyBeforeAttack`))
      (`Planet.SendUnitsToTarget` _array_element (`self.GetClosestNotOwnedPlanet` (`self.K2_GetActorLocation` _array_element)))
      (break))))

(fn `GetClosestNotOwnedPlanet`
  (params (Location :type "Vector Structure"))
  (returns (ClosestPlanet :type "Planet Object Reference"))
  (locals (LocationToTest :type "Vector Structure") (CurrentClosestPlanet :type "Planet Object Reference") (CurrentClosestDistance :type "Float (double-precision)"))
  (set `local.LocationToTest` Location)
  (set `local.CurrentClosestDistance` 0.0)
  (for _array_element (`self.NotOwnedPlanets`)
    (bind _returnvalue (`KismetMathLibrary.VSize` (- (`self.K2_GetActorLocation` _array_element) (`local.LocationToTest`))))
    (if (< _returnvalue (`local.CurrentClosestDistance`))
      (set `local.CurrentClosestPlanet` _array_element)
      (set `local.CurrentClosestDistance` _returnvalue)))
  (return (`local.CurrentClosestPlanet`)))

(fn `GetPlanetOccupancyRatio`
  (params (Planet :type "Planet Object Reference"))
  (returns (Occupancy :type "Float (double-precision)"))
  (return (/ (`KismetMathLibrary.Conv_IntToDouble` (`Planet.CurrentUnits` Planet)) (`KismetMathLibrary.Conv_IntToDouble` (`Planet.MaxUnits` Planet)))))

(fn `UserConstructionScript`)