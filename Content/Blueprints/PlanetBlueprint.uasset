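; Planet actor Blueprint that toggles its selected state and a visual selection indicator.
; On BeginPlay it enables input from the first player controller, so Space Bar alternates between the Select and Deselect events through a FlipFlop.
; Each event sets IsSelected and applies it to the Selection component's visibility without propagating to children.
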(event `self.ReceiveBeginPlay`
  (`self.EnableInput` (`GameplayStatics.GetPlayerController` 0)))

(event `Key|SpaceBar`
  (params (Key :type "Key Structure"))
  (:`Pressed`
    (`/Engine/EditorBlueprintResources/StandardMacros.FlipFlop`
      (:`A`
        (`self.Select`))
      (:`B`
        (`self.Deselect`)))))

(event `Select`
  ;[1 1 1] Select and Deselect
  (bind _output_get (set `self.IsSelected` true))
  (`SceneComponent.SetVisibility` (`self.Selection`) _output_get false))

(event `Deselect`
  ;[1 1 1] Select and Deselect
  (bind _output_get (set `self.IsSelected` false))
  (`SceneComponent.SetVisibility` (`self.Selection`) _output_get false))

(fn `UserConstructionScript`)